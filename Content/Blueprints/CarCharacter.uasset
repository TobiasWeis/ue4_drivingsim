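; Car character that drives along the spline of a referenced SplineBlueprint and destroys itself at the end.
; BeginPlay resets the distance, then it and Tick place and rotate the capsule at that distance, using world location but local-space rotation.
; Distance grows by Speed each frame, without delta-time scaling.
; The construction script adds an offset static mesh component with a random mesh from the Meshes array.
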(event EventBeginPlay
  (bind _spline_blueprint (Variables|Default|GetSpline_Blueprint))
  (bind _spline (Variables|/Game/Blueprints/Spline.Spline_C|GetSpline _spline_blueprint))
  (Variables|Default|SetDistance%20Along%20Spine 0.0)
  (Transformation|SetWorldLocation (Variables|Collision|GetCapsuleComponent) (Spline|GetLocationatDistanceAlongSpline _spline (Variables|Default|GetDistance%20Along%20Spine) "World") false false)
  (Transformation|SetWorldRotation (Variables|Collision|GetCapsuleComponent) (Spline|GetRotationatDistanceAlongSpline _spline (Variables|Default|GetDistance%20Along%20Spine) "Local") false false)
  (Variables|Default|SetDistance%20Along%20Spine (+ (Variables|Default|GetDistance%20Along%20Spine) (Variables|Default|GetSpeed)))
  (if (>= (Variables|Default|GetDistance%20Along%20Spine) (Spline|GetSplineLength _spline))
    (Actor|DestroyActor)))

(event Collision|EventActorBeginOverlap
  (params (OtherActor :type Actor%20Object%20Reference)))

(event EventTick
  (params (DeltaSeconds :type Float%20%28single-precision%29))
  (bind _spline_blueprint (Variables|Default|GetSpline_Blueprint))
  (bind _spline (Variables|/Game/Blueprints/Spline.Spline_C|GetSpline _spline_blueprint))
  (Transformation|SetWorldLocation (Variables|Collision|GetCapsuleComponent) (Spline|GetLocationatDistanceAlongSpline _spline (Variables|Default|GetDistance%20Along%20Spine) "World") false false)
  (Transformation|SetWorldRotation (Variables|Collision|GetCapsuleComponent) (Spline|GetRotationatDistanceAlongSpline _spline (Variables|Default|GetDistance%20Along%20Spine) "Local") false false)
  (Variables|Default|SetDistance%20Along%20Spine (+ (Variables|Default|GetDistance%20Along%20Spine) (Variables|Default|GetSpeed)))
  (if (>= (Variables|Default|GetDistance%20Along%20Spine) (Spline|GetSplineLength _spline))
    (Actor|DestroyActor)))

(fn ConstructionScript
  (bind _returnvalue (AddComponent|AddStaticMeshComponent false (Math|Transform|MakeTransform "0, 0,-90.000000" "0,-90.000000, 0")))
  (Components|StaticMesh|SetStaticMesh _returnvalue (.Random%20Element (Utilities|GetRandomArrayElemnt (Variables|Default|GetMeshes)))))